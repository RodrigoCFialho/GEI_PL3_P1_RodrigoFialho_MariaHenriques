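; BP_Lock is a combination lock puzzle with three rotating, four-position dials that opens when its icons match the code.
; Turn toggles activation through BPI_Activable on itself, player pawn input and a blend between static and player cameras.
; While active, W/S move a material highlight between dials and A/D rotate the selected one.
; A dial landing on its code value triggers the full-array check, which plays the LockOpening timeline.
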(event EventBeginPlay)

(event Collision|EventActorBeginOverlap
  (params (OtherActor :type Actor%20Object%20Reference)))

(event EventTick
  (params (DeltaSeconds :type Float%20%28single-precision%29)))

(event EventToggleActivation
  (params (bActivate :type Boolean))
  (Variables|Default|SetbActive bActivate)
  (Development|PrintString (Utilities|String|Append "Is Active" (Utilities|String|ToString(Boolean) bActivate)))
  (Utilities|HighlightSelected))

(event Input|KeyboardEvents|W
  (params (Key :type Key%20Structure :default "None"))
  (:Pressed
    (Utilities|MoveUp)))

(event Input|KeyboardEvents|S
  (params (Key :type Key%20Structure :default "None"))
  (:Pressed
    (Utilities|MoveDown)))

(event Input|KeyboardEvents|D
  (params (Key :type Key%20Structure :default "None"))
  (bind _lockrotationpoint (Variables|Default|GetLockRotationPoint))
  (bind _returnvalue (Transformation|GetRelativeTransform _lockrotationpoint))
  (:Pressed
    (Utilities|MoveRight
      (:Out
        ;[1 1 1] Opening Lock
        (Development|PrintString "Unlocked")
        (if (Utilities|Array|Identical (Variables|Default|GetCode) (Variables|Default|GetIconValue))
          (Development|PrintString "Open")
          (bind (_direction _height _rotation) (Timeline|LockOpening PlayFromStart)
            (:Update
              (Transformation|SetRelativeLocationAndRotation _lockrotationpoint (Math|Vector|MakeVector (.x (.location _returnvalue)) (.y (.location _returnvalue)) _height) (Math|Rotator|MakeRotator 0.0 0.0 _rotation) false false))))))))

(event Input|KeyboardEvents|A
  (params (Key :type Key%20Structure :default "None"))
  (bind _lockrotationpoint (Variables|Default|GetLockRotationPoint))
  (bind _returnvalue (Transformation|GetRelativeTransform _lockrotationpoint))
  (:Pressed
    (Utilities|MoveLeft
      (:Out
        ;[1 1 1] Opening Lock
        (Development|PrintString "Unlocked")
        (if (Utilities|Array|Identical (Variables|Default|GetCode) (Variables|Default|GetIconValue))
          (Development|PrintString "Open")
          (bind (_direction _height _rotation) (Timeline|LockOpening PlayFromStart)
            (:Update
              (Transformation|SetRelativeLocationAndRotation _lockrotationpoint (Math|Vector|MakeVector (.x (.location _returnvalue)) (.y (.location _returnvalue)) _height) (Math|Rotator|MakeRotator 0.0 0.0 _rotation) false false))))))))

(fn ConstructionScript
  (bind _lockcoderow (Variables|Default|GetLockCodeRow))
  (Utilities|Array|Clear _lockcoderow)
  (Utilities|Array|Add _lockcoderow (Variables|Default|GetLockCode1))
  (Utilities|Array|Add _lockcoderow (Variables|Default|GetLockCode2))
  (Utilities|Array|Add _lockcoderow (Variables|Default|GetLockCode3)))

(fn Turn
  (params (bOn :type Boolean))
  (|CallParentFunction bOn)
  (Utilities|Interact bOn
    (:Out
      (if bOn
        (Utilities|ToggleCharacterMovement false
          (:Out
            (Utilities|ChangeViewtoStaticCamera)))
        (else
          (Utilities|ToggleCharacterMovement true
            (:Out
              (Utilities|ChangeViewtoControllerCamera))))))))