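; BP_Blockade is a blockade actor linked to three void orbs, which the construction script gathers into the VoidOrbs array.
; Tick counts invalid orb entries into a counter that is never reset, so one missing orb raises it again every frame.
; The check for a count of three leads to nothing, and the DestroyActor node is unconnected, so the blockade never removes itself here.
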(event EventBeginPlay)

(event Collision|EventActorBeginOverlap
  (params (OtherActor :type Actor%20Object%20Reference)))

(event EventTick
  (params (DeltaSeconds :type Float%20%28single-precision%29))
  (for _array_element (Variables|Default|GetVoidOrbs)
    (Utilities|IsValid _array_element
      (:Is%20Not%20Valid
        (bind _output_get (Variables|Default|Setyes (+ (Variables|Default|Getyes) 1)))
        (if (== _output_get 3)
          _)))))

(fn ConstructionScript
  (bind _voidorbs (Variables|Default|GetVoidOrbs))
  (Utilities|Array|Clear _voidorbs)
  (Utilities|Array|Add _voidorbs (Variables|Default|GetVoidOrb))
  (Utilities|Array|Add _voidorbs (Variables|Default|GetVoidOrb1))
  (Utilities|Array|Add _voidorbs (Variables|Default|GetVoidOrb2)))