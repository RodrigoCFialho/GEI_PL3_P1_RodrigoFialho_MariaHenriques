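; BP_VoidOrb is an orb actor that activates, dissolves and destroys itself when the E key is pressed.
; The key press calls Turn, which runs the parent's Turn and then Interact, toggling activation through a BPI_Activable cast on itself.
; A Dissolve timeline then drives the Opacity parameter on the Sphere's materials and destroys the actor when finished.
; The E input has no overlap or proximity check.
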(event EventBeginPlay)

(event Collision|EventActorBeginOverlap
  (params (OtherActor :type Actor%20Object%20Reference)))

(event EventTick
  (params (DeltaSeconds :type Float%20%28single-precision%29)))

(event Input|KeyboardEvents|E
  (params (Key :type Key%20Structure :default "None"))
  (:Pressed
    (CallFunction|Turn true)
    (bind _dissolve (Timeline|Dissolve Play)
      (:Update
        (Rendering|Material|SetScalarParameterValueonMaterials (Variables|Default|GetSphere) "Opacity" _dissolve))
      (:Finished
        (Actor|DestroyActor)))))

(fn ConstructionScript)

(fn Turn
  (params (bOn :type Boolean))
  (|CallParentFunction bOn)
  (Utilities|Interact bOn))