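; BP_GeneralSwitch is a switch that toggles a linked actor and hands the player's view to a camera while it is on.
; Turn calls the parent implementation, then passes the state to ActorToActivate through the BPI_Activable interface.
; Turning on disables the controlled pawn's input and sets the view target to Camera.
; Turning off re-enables input and returns the view to the player character.
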(event EventBeginPlay)

(event Collision|EventActorBeginOverlap
  (params (OtherActor :type Actor%20Object%20Reference)))

(event EventTick
  (params (DeltaSeconds :type Float%20%28single-precision%29)))

(fn ConstructionScript)

(fn Turn
  (params (bOn :type Boolean))
  (|CallParentFunction bOn)
  (Utilities|ToggleSwitch bOn
    (:Out
      (if bOn
        (Utilities|ToggleCharacterMovement false
          (:Out
            (Utilities|ChangeViewtoStaticCamera)))
        (else
          (Utilities|ToggleCharacterMovement true
            (:Out
              (Utilities|ChangeViewtoControllerCamera))))))))